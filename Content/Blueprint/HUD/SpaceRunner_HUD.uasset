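; SpaceRunner HUD that sets up the game's UI and a timed turbo tutorial on BeginPlay.
; It creates a main menu widget without adding it to the viewport, then displays the SpaceRunner main widget.
; After a fixed delay it pauses the game, shows the turbo tutorial widget and spawns a BP_TurboDim actor at a hardcoded world location.
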(event `self.ReceiveBeginPlay`
  ;[1 1 1] Main Menù
  (`|CreateWidget` "/Game/Blueprint/HUD/WidgetBlueprint/MainMenuWidget.MainMenuWidget_C")
  ;[1 1 1] Event Begin Play {Main widget}
  (bind _returnvalue (`|CreateWidget` "/Game/Blueprint/HUD/WidgetBlueprint/SpaceRunner_MainWidget.SpaceRunner_MainWidget_C" (`GameplayStatics.GetPlayerController` 0)))
  (`UserWidget.AddToViewport` _returnvalue 0)
  (`KismetSystemLibrary.Delay` 15.0)
  (`GameplayStatics.SetGamePaused` true)
  ;[1 1 1] Tutorial
  (bind _returnvalue_2 (`|CreateWidget` "/Game/Blueprint/HUD/WidgetBlueprint/TutorialBlueprint_Turbo.TutorialBlueprint_Turbo_C" (`GameplayStatics.GetPlayerController` 0)))
  (`UserWidget.AddToViewport` _returnvalue_2 0)
  (`|SpawnActorFromClass` "/Game/Blueprint/PickUp-Items/BP_TurboDim.BP_TurboDim_C" (`KismetMathLibrary.MakeTransform` (1011114.1875 -131189.0 -3387.999268) (struct)) "Undefined" "OverrideRootScale"))

(fn `UserConstructionScript`)