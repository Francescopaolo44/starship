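; Stage one level actor that populates an asteroid field with obstacles and TurboDim actors at game start.
; On BeginPlay, four functions each run a fixed loop spawning asteroid residues, asteroids, big asteroids and TurboDim.
; Every spawn gets a random position inside the AsteroidArea box, offset by the actor's location, plus a random rotation.
; Asteroid types get random non-uniform scale in ranges that grow by type, while TurboDim uses a fixed scale.
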(event `self.ReceiveBeginPlay`
  ;[1 1 1] Begin Play
  (`self.Spawn Residues_of_Asteroid`)
  (`self.Spawn Asteroid`)
  (`self.Spawn Big Asteroid`)
  (`self.Spawn TurboDim`))

(fn `Spawn Asteroid`
  (bind _returnvalue (`KismetMathLibrary.RandomFloatInRange` 10.0 200.0))
  (bind _x (.x (`BoxComponent.GetScaledBoxExtent` (`self.Asteroid Area`))))
  (bind _y (.y (`BoxComponent.GetScaledBoxExtent` (`self.Asteroid Area`))))
  (bind _z (.z (`BoxComponent.GetScaledBoxExtent` (`self.Asteroid Area`))))
  ;[1 1 1] Asteroid Spawn
  (for _ (range 81)
    (`|SpawnActorFromClass` "/Game/Blueprint/Stage/1_Stage/BP_AsteroidObstacle.BP_AsteroidObstacle_C" (`KismetMathLibrary.MakeTransform` (+ (`KismetMathLibrary.MakeVector` (`KismetMathLibrary.RandomFloatInRange` (* _x -1.0) _x) (`KismetMathLibrary.RandomFloatInRange` (* _y -1.0) _y) (`KismetMathLibrary.RandomFloatInRange` (* _z -1.0) _z)) (`self.K2_GetActorLocation`)) (`KismetMathLibrary.RandomRotator` true) (`KismetMathLibrary.MakeVector` _returnvalue _returnvalue _returnvalue)) "Undefined" "OverrideRootScale")))

(fn `Spawn Big Asteroid`
  (bind _returnvalue (`KismetMathLibrary.RandomFloatInRange` 100.0 500.0))
  (bind _x (.x (`BoxComponent.GetScaledBoxExtent` (`self.Asteroid Area`))))
  (bind _y (.y (`BoxComponent.GetScaledBoxExtent` (`self.Asteroid Area`))))
  (bind _z (.z (`BoxComponent.GetScaledBoxExtent` (`self.Asteroid Area`))))
  ;[1 1 1] Asteroid Spawn
  (for _ (range 31)
    (`|SpawnActorFromClass` "/Game/Blueprint/Stage/1_Stage/BP_BigAsteroid.BP_BigAsteroid_C" (`KismetMathLibrary.MakeTransform` (+ (`KismetMathLibrary.MakeVector` (`KismetMathLibrary.RandomFloatInRange` (* _x -1.0) _x) (`KismetMathLibrary.RandomFloatInRange` (* _y -1.0) _y) (`KismetMathLibrary.RandomFloatInRange` (* _z -1.0) _z)) (`self.K2_GetActorLocation`)) (`KismetMathLibrary.RandomRotator` true) (`KismetMathLibrary.MakeVector` _returnvalue _returnvalue _returnvalue)) "Undefined" "OverrideRootScale")))

(fn `Spawn Residues_of_Asteroid`
  (bind _returnvalue (`KismetMathLibrary.RandomFloatInRange` 1.0 20.0))
  (bind _x (.x (`BoxComponent.GetScaledBoxExtent` (`self.Asteroid Area`))))
  (bind _y (.y (`BoxComponent.GetScaledBoxExtent` (`self.Asteroid Area`))))
  (bind _z (.z (`BoxComponent.GetScaledBoxExtent` (`self.Asteroid Area`))))
  ;[1 1 1] Residues of Asteroid Spawn
  (for _ (range 1001)
    (`|SpawnActorFromClass` "/Game/Blueprint/Stage/1_Stage/BP_Residues_of_AsteroidObstacles.BP_Residues_of_AsteroidObstacles_C" (`KismetMathLibrary.MakeTransform` (+ (`KismetMathLibrary.MakeVector` (`KismetMathLibrary.RandomFloatInRange` (* _x -1.0) _x) (`KismetMathLibrary.RandomFloatInRange` (* _y -1.0) _y) (`KismetMathLibrary.RandomFloatInRange` (* _z -1.0) _z)) (`self.K2_GetActorLocation`)) (`KismetMathLibrary.RandomRotator` true) (`KismetMathLibrary.MakeVector` _returnvalue _returnvalue _returnvalue)) "Undefined" "OverrideRootScale")))

(fn `Spawn TurboDim`
  (bind _x (.x (`BoxComponent.GetScaledBoxExtent` (`self.Asteroid Area`))))
  (bind _y (.y (`BoxComponent.GetScaledBoxExtent` (`self.Asteroid Area`))))
  (bind _z (.z (`BoxComponent.GetScaledBoxExtent` (`self.Asteroid Area`))))
  ;[1 1 1] TurboDim Spawn
  (for _ (range 201)
    (`|SpawnActorFromClass` "/Game/Blueprint/PickUp-Items/BP_TurboDim.BP_TurboDim_C" (`KismetMathLibrary.MakeTransform` (+ (`KismetMathLibrary.MakeVector` (`KismetMathLibrary.RandomFloatInRange` (* _x -1.0) _x) (`KismetMathLibrary.RandomFloatInRange` (* _y -1.0) _y) (`KismetMathLibrary.RandomFloatInRange` (* _z -1.0) _z)) (`self.K2_GetActorLocation`)) (`KismetMathLibrary.RandomRotator` true) (2.0 2.0 2.0)) "Undefined" "OverrideRootScale")))

(fn `UserConstructionScript`)